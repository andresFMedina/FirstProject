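; Player controller Blueprint that animates the pause menu as it is shown and hidden.
; It extends the parent's display and hide events, calling the parent logic first, then casting the inherited menu reference to PauseMenu_WBP.
; Showing plays the menu animation forward; hiding plays the same animation in reverse and sets the widget hidden after a short fixed delay.
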(event EventHidePauseMenu
  (|CallParentFunction)
  (bind _aspause_menu_wbp (Utilities|Casting|CastToPauseMenu_WBP (Variables|Default|GetPauseMenu)))
  (UserInterface|Animation|PlayAnimation _aspause_menu_wbp (Variables|/Game/HUD/PauseMenu_WBP.PauseMenu_WBP_C|GetPauseMenuAnimation _aspause_menu_wbp) 0.0 1 "Reverse" 1.0 false)
  (Utilities|FlowControl|Delay 0.25)
  (Widget|SetVisibility (Variables|Default|GetPauseMenu) "Hidden"))

(event EventDisplayPauseMenu
  (|CallParentFunction)
  (bind _aspause_menu_wbp (Utilities|Casting|CastToPauseMenu_WBP (Variables|Default|GetPauseMenu)))
  (UserInterface|Animation|PlayAnimation _aspause_menu_wbp (Variables|/Game/HUD/PauseMenu_WBP.PauseMenu_WBP_C|GetPauseMenuAnimation _aspause_menu_wbp) 0.0 1 "Forward" 1.0 false))

(fn ConstructionScript)